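; Monster character Blueprint with goblin animations that chases and melee-attacks the player, then drops loot on death.
; Each Tick measures player distance and direction to drive an idle, follow and attack state machine, idling when the player is dead.
; Attack events toggle a capsule hitbox that applies damage on overlap, and attack end either repeats the slash or resumes the chase.
; Damage briefly swaps the mesh material; death spawns an item and weapon after a delay.
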(event `OncollStart_Attack`
  ;[1 1 1] CapsuleCollision Activation Start&End
  (`PrimitiveComponent.SetCollisionEnabled` (`self.Capsule`) "QueryAndPhysics"))

(event `OnCollEnd_Attack`
  ;[1 1 1] CapsuleCollision Activation Start&End
  (`PrimitiveComponent.SetCollisionEnabled` (`self.Capsule`) "NoCollision"))

(event `self.Capsule.OnComponentBeginOverlap`
  (params (OverlappedComponent :type "PrimitiveComponent Object Reference") (OtherActor :type "Actor Object Reference") (OtherComp :type "PrimitiveComponent Object Reference") (OtherBodyIndex :type Integer) (bFromSweep :type Boolean) (SweepResult :type "HitResult Structure (by ref)"))
  ;[1 1 1] SetAttackDamage
  (if (!= OtherActor self)
    (`GameplayStatics.ApplyDamage` OtherActor (`self.Atk`) null self)))

(event `OnAnimEnd_Attack`
  ;[1 1 1] AttackEnd After Attack or Follow
  (set `self.IsAttacking` false)
  (if (`self.IsDeathPlayerCharacter`)
    (set `self.CurState` "NewEnumerator3")
    (elif (> (`self.DistancePlayerCharacter`) 180.0)
      (set `self.CurState` "NewEnumerator1")
      (else
        (`self.PlayAnimMontage` "/Game/Monsster/Goblin_slash_Montage.Goblin_slash_Montage")
        (set `self.IsAttacking` true)))))

(event `self.ReceiveTick`
  (params (DeltaSeconds :type "Float (single-precision)"))
  ;[1 1 1] Idle/Attack/Follow
  (`self.SaveDistAndDir`)
  (if (`self.IsDeathPlayerCharacter`)
    (set `self.CurState` "NewEnumerator3"))
  (switch `/Game/Monsster/MonsterState` (`self.CurState`)
    (:`NewEnumerator0`
      (if (<= (`self.DistancePlayerCharacter`) 500.0)
        (set `self.CurState` "NewEnumerator1")))
    (:`NewEnumerator1`
      (if (<= (`self.DistancePlayerCharacter`) 160.0)
        (set `self.CurState` "NewEnumerator2")
        (`self.PlayAnimMontage` "/Game/Monsster/Goblin_slash_Montage.Goblin_slash_Montage")
        (set `self.IsAttacking` true)
        (else
          (`self.AddMovementInput` (`self.DirToPlayerCharacter`)))))
    (:`NewEnumerator2`
      (if (`self.IsAttacking`)
        _
        (elif (> (`self.DistancePlayerCharacter`) 180.0)
          (set `self.CurState` "NewEnumerator1"))))))

(event `SaveDistAndDir`
  (bind _returnvalue (`GameplayStatics.GetPlayerCharacter` 0))
  (bind _returnvalue_2 (`KismetMathLibrary.MakeVector` (.x (- (`self.K2_GetActorLocation` _returnvalue) (`self.K2_GetActorLocation`))) (.y (- (`self.K2_GetActorLocation` _returnvalue) (`self.K2_GetActorLocation`))) (.z (- (`self.K2_GetActorLocation` _returnvalue) (`self.K2_GetActorLocation`)))))
  ;[1 1 1] PlayerMonsterDistance&Direction
  (bind _asmove_char_bp (cast `/Game/MoveCharBP` _returnvalue))
  (set `self.IsDeathPlayerCharacter` (`/Game/MoveCharBP.IsDeath` _asmove_char_bp))
  (set `self.DistancePlayerCharacter` (`KismetMathLibrary.VSize` _returnvalue_2))
  (set `self.DirToPlayerCharacter` (`KismetMathLibrary.Normal` _returnvalue_2)))

(event `self.ReceiveAnyDamage`
  (params (Damage :type "Float (single-precision)") (DamageType :type "DamageType Object Reference") (InstigatedBy :type "Controller Object Reference") (DamageCauser :type "Actor Object Reference"))
  ;[1 1 1] DamageEvent
  (bind _output_get (set `self.HP` (- (`self.HP`) Damage)))
  (`self.ChangeDamageColor`)
  (if (<= _output_get 0.0)
    (`self.PlayAnimMontage` "/Game/Monsster/Goblin_Death_Montage.Goblin_Death_Montage")
    (set `self.CurState` "NewEnumerator4")
    ;[1 1 1] DeathAfterItemDrop
    (`PrimitiveComponent.SetCollisionEnabled` (`self.CapsuleComponent`) "NoCollision")
    (`PrimitiveComponent.SetCollisionEnabled` (`self.Capsule`) "NoCollision")
    (`KismetSystemLibrary.Delay` 4.1)
    (`|SpawnActorFromClass` "/Game/Monsster/BP_Item.BP_Item_C" (`self.GetTransform`) "Undefined" "OverrideRootScale" null null)
    (`|SpawnActorFromClass` "/Game/Monsster/BP_Weapon.BP_Weapon_C" (`KismetMathLibrary.MakeTransform` (`KismetMathLibrary.MakeVector` (+ (.x (.location (`self.GetTransform`))) 0.0) (+ (.y (.location (`self.GetTransform`))) 200.0) (+ (.z (.location (`self.GetTransform`))) 0.0))) "Undefined" "OverrideRootScale" null null)
    (`self.K2_DestroyActor`)))

(event `ChangeDamageColor`
  ;[1 1 1] ChangeDamageColor
  (`PrimitiveComponent.SetMaterial` (`self.Mesh`) 1 "/Game/Monsster/phong1_Inst.phong1_Inst")
  (`KismetSystemLibrary.Delay` 0.2)
  (`PrimitiveComponent.SetMaterial` (`self.Mesh`) 1 "/Game/Monsster/phong1.phong1"))

(fn `UserConstructionScript`)