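; MoveCharBP is the player character, with movement, a punch attack and object interaction.
; Axis inputs move it along fixed world axes, and on BeginPlay the player's view switches to Cam.
; Left click plays a punch montage, while any overlap with another actor applies Atk damage, independent of the punch.
; E sends OnInteractMessage to CurrentInteract, which interactable objects set externally when the player is in range.
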(event `Key|LeftMouseButton`
  (params (Key :type "Key Structure"))
  (:`Pressed`
    (`self.PlayAnimMontage` "/Game/Punching_Anim_Montage.Punching_Anim_Montage")))

(event `InputAxis|LeftRight`
  (params (AxisValue :type "Float (single-precision)"))
  (`self.AddMovementInput` (0.0 1.0 0.0) AxisValue))

(event `self.ReceiveBeginPlay`
  (`PlayerController.SetViewTargetWithBlend` (`GameplayStatics.GetPlayerController` 0) (`self.Cam`) 0.0 "VTBlend_Linear" 0.0 false))

(event `InputAxis|FowardBackward`
  (params (AxisValue :type "Float (single-precision)"))
  (`self.AddMovementInput` (1.0 0.0 0.0) AxisValue))

(event `self.ReceiveActorBeginOverlap`
  (params (OtherActor :type "Actor Object Reference"))
  (if (not (== OtherActor self))
    (`GameplayStatics.ApplyDamage` OtherActor (`self.Atk`) null self)))

(event `Key|E`
  (params (Key :type "Key Structure"))
  (bind _current_interact (`self.Current interact`))
  ;[1 1 1] If the player has walked in range of an interact object,
  ; then the variable here will be set extemally from the blueprint of the
  ; interact object
  (:`Pressed`
    (`/Engine/EditorBlueprintResources/StandardMacros.IsValid` _current_interact
      (:`Is Valid`
        (message `/Game/Campfire/Interact_BPI.On interact` _current_interact)))))

(fn `UserConstructionScript`)